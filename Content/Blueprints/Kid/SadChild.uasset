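; Sad child actor that plays a random joke with on-screen text and audio when the player enters its trigger box.
; A DoOnce-gated overlap flags the player as ByKid and shows the joke widget, then its punchline after a delay.
; The last joke is a special single clip without punchline, and only the other jokes re-arm the trigger.
; Each joke ends by enabling ContinueAvailable and showing an F-key prompt.
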(event `ResetDoOnce`
  (bind _randomnum (`self.RandomNum`))
  (bind _asbp_player (cast `/Game/Blueprints/Player/BP_Player` (`GameplayStatics.GetPlayerCharacter` 0) :!pure true))
  (goto _label :!via `Reset`))

(event `self.Box.OnComponentBeginOverlap`
  (params (OverlappedComponent :type "PrimitiveComponent Object Reference") (OtherActor :type "Actor Object Reference") (OtherComp :type "PrimitiveComponent Object Reference") (OtherBodyIndex :type Integer) (bFromSweep :type Boolean) (SweepResult :type "HitResult Structure (by ref)"))
  (bind _randomnum (`self.RandomNum`))
  (bind _asbp_player (cast `/Game/Blueprints/Player/BP_Player` (`GameplayStatics.GetPlayerCharacter` 0) :!pure true))
  (`/Engine/EditorBlueprintResources/StandardMacros.DoOnce` false :!label _label
    (:`Completed`
      (bind _asbp_player_2 (cast `/Game/Blueprints/Player/BP_Player` OtherActor))
      (set `/Game/Blueprints/Player/BP_Player.ByKid` true _asbp_player_2)
      (bind _output_get (set `self.RandomNum` (`KismetMathLibrary.RandomIntegerInRange` 0 6)))
      (if (== _output_get 6)
        (set `/Game/Blueprints/Player/BP_Player.DisplayText` (`KismetTextLibrary.Conv_StringToText` (`|GetArrayItem` (`self.FunnyJokes`) 6)) _asbp_player_2)
        (bind _returnvalue (`|CreateWidget` "/Game/Blueprints/BPWidgets/WB_JokeText.WB_JokeText_C"))
        (`UserWidget.AddToViewport` _returnvalue 0)
        (`GameplayStatics.PlaySound2D` "/Game/Audio/Jokes/Joke_04.Joke_04" 1.0 1.0 0.0 null null)
        (`KismetSystemLibrary.Delay` 8.1)
        (`Widget.RemoveFromParent` _returnvalue)
        (set `/Game/Blueprints/Player/BP_Player.ContinueAvailable` true _asbp_player)
        (bind _returnvalue_2 (`|CreateWidget` "/Game/Blueprints/BPWidgets/WB_FKeyPrompt.WB_FKeyPrompt_C"))
        (`UserWidget.AddToViewport` _returnvalue_2 0)
        (else
          (set `/Game/Blueprints/Player/BP_Player.DisplayText` (`KismetTextLibrary.Conv_StringToText` (`|GetArrayItem` (`self.FunnyJokes`) _output_get)) _asbp_player_2)
          (bind _returnvalue_3 (`|CreateWidget` "/Game/Blueprints/BPWidgets/WB_JokeText.WB_JokeText_C"))
          (`UserWidget.AddToViewport` _returnvalue_3 0)
          (`GameplayStatics.PlaySound2D` (`|GetArrayItem` (`self.Jokearray`) _randomnum) 1.0 1.0 0.0 null null)
          (`KismetSystemLibrary.Delay` 3.1)
          (set `/Game/Blueprints/Player/BP_Player.DisplayText` (`KismetTextLibrary.Conv_StringToText` (`|GetArrayItem` (`self.Punchlines`) _output_get)) _asbp_player_2)
          (`GameplayStatics.PlaySound2D` (`|GetArrayItem` (`self.punchlinearray`) _randomnum) 1.0 1.0 0.0 null null)
          (`KismetSystemLibrary.Delay` 2.3)
          (`Widget.RemoveFromParent` _returnvalue_3)
          (`self.ResetDoOnce`)
          (set `/Game/Blueprints/Player/BP_Player.ContinueAvailable` true _asbp_player)
          (bind _returnvalue_4 (`|CreateWidget` "/Game/Blueprints/BPWidgets/WB_FKeyPrompt.WB_FKeyPrompt_C"))
          (`UserWidget.AddToViewport` _returnvalue_4 0))))))

(fn `UserConstructionScript`)