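; BP_Door is a Paper2D door that opens when the player holds a key.
; Interact casts the player character to BP_Player and reads its HasKey, then plays the DoorOpen flipbook once and disables PlayerBlocker collision, or prints "No Key".
; A separate PickUpKey event sets the door's own HasKey, which Interact does not read.
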(event `/Game/Blueprints/DoorSystem/BPI_Interact.Interact`
  (bind _paperflipbook (`self.PaperFlipbook`))
  (if (`/Game/Blueprints/Player/BP_Player.HasKey?` (cast `/Game/Blueprints/Player/BP_Player` (`GameplayStatics.GetPlayerCharacter` 0) :!pure true))
    (`PaperFlipbookComponent.SetLooping` _paperflipbook false)
    (`PaperFlipbookComponent.SetFlipbook` _paperflipbook "/Game/Assets/Door_Sprite/DoorOpen.DoorOpen")
    (`PrimitiveComponent.SetCollisionEnabled` (`self.PlayerBlocker`) "NoCollision")
    (else
      (`KismetSystemLibrary.PrintString` "No Key"))))

(event `/Game/Blueprints/DoorSystem/BPI_Door.Pick Up Key`
  (set `self.HasKey?` true))

(fn `UserConstructionScript`)